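; BP_PlayerControllerArena is a player controller that toggles a weapon spawn widget on the SpawnWidget input action.
; When none is open, it creates a SpawnWeapon widget, adds it to the viewport, focuses it in Game and UI input mode and shows the cursor.
; Pressing again removes the widget, clears the stored reference, restores game-only input and hides the cursor.
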(event Input|ActionEvents|InputActionSpawnWidget
  (params (Key :type Key%20Structure :default "None"))
  (bind _self self)
  (:Pressed
    (Utilities|IsValid (Variables|Default|GetSpawnWidget)
      (:Is%20Valid
        (Widget|RemovefromParent (Variables|Default|GetSpawnWidget))
        (Input|SetInputModeGameOnly _self)
        (Variables|Default|SetSpawnWidget 0)
        (Variables|Default|SetbShowMouseCursor false))
      (:Is%20Not%20Valid
        (bind _returnvalue (UserInterface|CreateWidget "/Game/UI/SpawnWeapon.SpawnWeapon_C" _self))
        (UserInterface|Viewport|AddtoViewport _returnvalue 0)
        (Variables|Default|SetSpawnWidget _returnvalue)
        (Input|SetInputModeGameandUI _self _returnvalue "DoNotLock" true)
        (Variables|Default|SetbShowMouseCursor true)))))

(fn ConstructionScript)
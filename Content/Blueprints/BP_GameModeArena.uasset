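; Arena game mode Blueprint that handles player respawning and weapon spawning.
; It caches all PlayerStarts at BeginPlay; respawning teleports the existing pawn to a random one, then restores BP_PlayerCharacter health and input.
; Weapon spawning runs only with authority, looks up the class by row name in DT_WeaponData, spawns it ahead of the requesting player's pawn and calls WasSpawned on it.
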(event EventRespawnCharacter
  (params (PlayerController :type Player%20Controller%20Object%20Reference))
  (bind _returnvalue (Pawn|GetControlledPawn PlayerController))
  (bind _playerstart (Variables|Default|GetPlayerStart))
  (Development|PrintString "Respawn Character")
  (Transformation|SetActorLocation _returnvalue (Transformation|GetActorLocation (Utilities|Array|Get(acopy) _playerstart (Math|Random|RandomIntegerinRange 0 (- (Utilities|Array|Length _playerstart) 1)))) false true)
  (bind _asbp_player_character (Utilities|Casting|CastToBP_PlayerCharacter _returnvalue))
  (Class|PlayerCharacter|SetHealth _asbp_player_character 1e+02)
  (Input|EnableInput _asbp_player_character PlayerController))

(event EventBeginPlay
  (bind _outactors (Actor|GetAllActorsOfClass "/Script/Engine.PlayerStart"))
  (Variables|Default|SetPlayerStart _outactors))

(event EventSpawnWeapon
  (params (RowName :type Name :default "None") (PlayerController :type Player%20Controller%20Arena%20Object%20Reference))
  (bind _returnvalue (Pawn|GetControlledPawn PlayerController))
  (Networking|SwitchHasAuthority
    (:Authority
      (bind _returnvalue_2 (Utilities|GetDataTableRow "/Game/AssetData/DataTable/DT_WeaponData.DT_WeaponData" RowName)
        (:then
          (bind _returnvalue_3 (Game|SpawnActorfromClass (.weaponclass _returnvalue_2) (Math|Transform|MakeTransform (+ (Transformation|GetActorLocation _returnvalue) (* (Transformation|GetActorForwardVector _returnvalue) 150)) "0, 0, 0" "1,1,1") "AlwaysSpawn" 0 RowName 0))
          (Class|WeaponBase|WasSpawned _returnvalue_3))))))

(fn ConstructionScript)